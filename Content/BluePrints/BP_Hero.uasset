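; BP_Hero is the hero Blueprint that sets up its inventory, on-screen UI and background music.
; The construction script initializes InventoryComponent.
; BeginPlay shows the Test and Test_bag widgets, prints the GameManager's current coin count, and creates W_Bag, storing it as the component's BagUI.
; It also starts a 2D BGM sound with auto-destroy off, keeping the audio reference.
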(event `self.ReceiveBeginPlay`
  (`|ExecutionSequence`
    (:`then_0`
      (bind _returnvalue (`|CreateWidget` "/Game/UI/test.test_C"))
      (`UserWidget.AddToViewport` _returnvalue 0)
      (`KismetSystemLibrary.PrintString` (`KismetStringLibrary.Conv_IntToString` (`/Game/BluePrints/Managers/BP_GameManager.curCoin` (`self.GameManagerRef`))))
      (bind _returnvalue_2 (`|CreateWidget` "/Game/UI/W_Bag.W_Bag_C"))
      (bind _output_get (set `/Game/BluePrints/InventoryComponent.BagUI` _returnvalue_2 (`self.InventoryComponent`)))
      (`UserWidget.AddToViewport` _output_get 0))
    (:`then_1`
      (bind _returnvalue_3 (`GameplayStatics.CreateSound2D` "/Game/Resources/MusicAndSounds/BGM.BGM" 1.0 1.0 0.0 null false false))
      (bind _output_get_2 (set `self.BGM` _returnvalue_3))
      (`AudioComponent.Play` _output_get_2 0.0))
    (:`then_2`
      (bind _returnvalue_4 (`|CreateWidget` "/Game/UI/test_bag.test_bag_C"))
      (`UserWidget.AddToViewport` _returnvalue_4 0))))

(fn `UserConstructionScript`
  (`/Game/BluePrints/InventoryComponent.InitInventoryComponent` (`self.InventoryComponent`)))