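; BP_Grid is a clickable farm plot that handles planting and harvesting of medicinal herbs.
; Clicks on the field or grown-plant sprite dispatch on plot state, gated by the GameManager's cursor state.
; Planting stores the selected seed and updates sprites through PlantsManager lookups; growth timing is not driven here.
; Harvesting clears sprites and inserts a mapped item index into the hero's bag, but leaves plot state unchanged, as the reset sits in disconnected legacy logic.
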(event `self.ReceiveBeginPlay`
  (bind _asbp_hero (cast `/Game/BluePrints/BP_Hero` (`GameplayStatics.GetPlayerCharacter` 0)))
  (set `self.HeroRef` _asbp_hero)
  (set `self.Game Manager Ref` (`/Game/BluePrints/BP_Hero.GameManagerRef` (`self.HeroRef`))))

(event `self.ReceiveActorOnClicked`
  (params (ButtonPressed :type "Key Structure")))

(event `self.MyField.OnClicked`
  (params (TouchedComponent :type "PrimitiveComponent Object Reference") (ButtonPressed :type "Key Structure"))
  (`KismetSystemLibrary.PrintString` (`|GetEnumeratorNameAsString` (`self.curState`)))
  (switch `/Game/EnumsAndStructs/GridState` (`self.curState`)
    (:`NewEnumerator0`
      (`self.OnClickedEmpty`))
    (:`NewEnumerator2`
      (`self.OnClickedGrown`))))

(event `self.GrownPlant.OnClicked`
  (params (TouchedComponent :type "PrimitiveComponent Object Reference") (ButtonPressed :type "Key Structure"))
  (switch `/Game/EnumsAndStructs/GridState` (`self.curState`)
    (:`NewEnumerator2`
      (`self.OnClickedGrown`))))

(fn `OnClickedEmpty`
  (if (`|EnumEquality` (`/Game/BluePrints/Managers/BP_GameManager.CursorState` (`self.Game Manager Ref`)) "NewEnumerator0")
    (set `self.curState` "NewEnumerator1")
    (set `self.curPlant` (`/Game/BluePrints/Managers/BP_GameManager.curSeed` (`self.Game Manager Ref`)))
    (`self.SetSpriteByStateAndPlant`)
    (`KismetSystemLibrary.PrintString` (`|GetEnumeratorNameAsString` (`self.curState`)))))

(fn `OnClickedGrown`
  (locals (static_CursorStateGain :type "/Game/EnumsAndStructs/CursorState Enum" :default "NewEnumerator1") (static_GrownState :type "/Game/EnumsAndStructs/GridState Enum" :default "NewEnumerator2"))
  (bind _heroref (`self.HeroRef`))
  ;[1 1 1] TO-DO :Use bag
  (if (== (`self.curState`) (`local.static_GrownState`))
    (if (`|EnumEquality` (`/Game/BluePrints/Managers/BP_GameManager.CursorState` (`self.Game Manager Ref`)) "NewEnumerator1")
      (`self.SetSprite` "/Game/Resources/Grids/单块土地_开垦__1__Sprite.单块土地_开垦__1__Sprite")
      (`PaperSpriteComponent.SetSprite` (`self.GrownPlant`) null)
      (bind _index (`self.PlantTypeToSeedIndex` (`self.curPlant`)))
      (`/Game/BluePrints/BP_Hero.InsertItem` _heroref _index 1 "NewEnumerator1")
      (`/Game/BluePrints/Managers/BP_BagManager.OutPutItems` (`/Game/BluePrints/BP_Hero.BagManagerRef` _heroref)))))

(fn `PlantTypeToName`
  (params (NewParam :type "/Game/EnumsAndStructs/Plants Enum" :default "NewEnumerator0"))
  (returns (NewParam1 :type Name))
  (switch `/Game/EnumsAndStructs/Plants` NewParam))

(fn `PlantTypeToSeedIndex`
  (params (type :type "/Game/EnumsAndStructs/Plants Enum" :default "NewEnumerator0"))
  (returns (index :type Integer))
  (switch `/Game/EnumsAndStructs/Plants` type
    (:`NewEnumerator3`
      (return 0))
    (:`NewEnumerator4`
      (return 3))
    (:`NewEnumerator5`
      (return 2))
    (:`NewEnumerator6`
      (return 1))
    (:`NewEnumerator7`
      (return 4))
    (:`NewEnumerator8`
      (return 2))
    (:`NewEnumerator9`
      (return 5))))

(fn `PropIndexToBagItem`
  (returns (NewParam :type "/Game/EnumsAndStructs/BagItem Structure"))
  (bind _curplant (`self.curPlant`))
  (return (make `/Game/EnumsAndStructs/BagItem` (`|GetEnumeratorName` _curplant) "NewEnumerator0" true 1 "成熟的向日葵" null null _curplant)))

(fn `SetSprite`
  (params (NewSprite :type "PaperSprite Object Reference"))
  (`PaperSpriteComponent.SetSprite` (`self.MyField`) NewSprite))

(fn `SetSpriteByStateAndPlant`
  (if (`|EnumEquality` (`self.curState`) "NewEnumerator3")
    (`PaperSpriteComponent.SetSprite` (`self.MyField`) "/Game/Resources/Grids/new单块土地_未开垦_Sprite.new单块土地_未开垦_Sprite")
    (elif (`|EnumEquality` (`self.curState`) "NewEnumerator0")
      (`PaperSpriteComponent.SetSprite` (`self.MyField`) "/Game/Resources/Grids/单块土地_开垦__1__Sprite.单块土地_开垦__1__Sprite")
      (else
        (bind _newparam (`/Game/BluePrints/Managers/BP_PlantInfoManager.FindInfoByPlantType` (`/Game/BluePrints/BP_Hero.PlantsManagerRef` (`self.HeroRef`)) (`self.curPlant`)))
        (switch `/Game/EnumsAndStructs/GridState` (`self.curState`)
          (:`NewEnumerator1`
            (`self.SetSprite` "/Game/Resources/Grids/单块土地_播种种子__1__Sprite.单块土地_播种种子__1__Sprite"))
          (:`NewEnumerator2`
            (`PaperSpriteComponent.SetSprite` (`self.GrownPlant`) (`.GrownIcon_13_82EE52964CE66F290E193A8A4370836F` (break `/Game/EnumsAndStructs/PlantsInfo` _newparam)))
            (`PaperSpriteComponent.SetSprite` (`self.MyField`) "/Game/Resources/Grids/单块土地_开垦__1__Sprite.单块土地_开垦__1__Sprite")))))))

(fn `UserConstructionScript`)