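; Bag manager that stores the player's seeds, medicinal materials and functional items in three maps of item ID to count.
; Insert routes by type to per-category functions that add to existing counts.
; Remove checks only the Functional map, then calls Insert with an unnegated count, so it adds.
; OutPutItems prints names and counts via BP_Hero lookups, with the seed and medicine lookups swapped.
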(event `self.ReceiveBeginPlay`
  (bind _asbp_hero (cast `/Game/BluePrints/BP_Hero` (`GameplayStatics.GetPlayerPawn` 0)))
  (set `self.As BP Hero` _asbp_hero))

(fn `CheckCanRemove`
  (params (id :type Integer) (num :type Integer))
  (returns (res :type Boolean))
  (bind (_value _returnvalue) (`BlueprintMapLibrary.Map_Find` (`self.Functional`) id))
  (if _returnvalue
    (if (< _value num)
      (return false)
      (else
        (return true)))
    (else
      (return false))))

(fn `Insert`
  (params (id :type Integer) (num :type Integer) (type :type "/Game/EnumsAndStructs/Item/PropType Enum" :default "NewEnumerator0"))
  (locals (ItemNum :type Integer) (SubBagToInsert :type "Map of Integer to Object Object Reference") (InId :type Integer) (InNum :type Integer))
  (bind _inid (`local.InId`))
  (bind _seeds (`self.Seeds`))
  (bind _inid_2 (`local.InId`))
  (bind _medic (`self.Medic`))
  (bind _inid_3 (`local.InId`))
  (bind _functional (`self.Functional`))
  (bind (_value _returnvalue) (`BlueprintMapLibrary.Map_Find` (`self.Seeds`) (`local.InId`)))
  (bind (_value_2 _returnvalue_2) (`BlueprintMapLibrary.Map_Find` (`self.Medic`) (`local.InId`)))
  (bind (_value_3 _returnvalue_3) (`BlueprintMapLibrary.Map_Find` (`self.Functional`) (`local.InId`)))
  (set `local.InId` id)
  (set `local.InNum` num)
  (switch `/Game/EnumsAndStructs/Item/PropType` type
    (:`NewEnumerator0`
      (if _returnvalue
        (bind _output_get (set `local.ItemNum` _value))
        (`BlueprintMapLibrary.Map_Remove` _seeds _inid)
        (`BlueprintMapLibrary.Map_Add` _seeds _inid (+ _output_get (`local.InNum`)))
        (else
          (`BlueprintMapLibrary.Map_Add` (`self.Seeds`) _inid (`local.InNum`))
          (`KismetSystemLibrary.PrintString` (`KismetStringLibrary.Conv_IntToString` (`BlueprintMapLibrary.Map_Length` (`self.Seeds`)))))))
    (:`NewEnumerator1`
      (if _returnvalue_2
        (bind _output_get_2 (set `local.ItemNum` _value_2))
        (`BlueprintMapLibrary.Map_Remove` _medic _inid_2)
        (`BlueprintMapLibrary.Map_Add` _medic _inid_2 (+ _output_get_2 (`local.InNum`)))
        (else
          (`BlueprintMapLibrary.Map_Add` (`self.Medic`) _inid_2 (`local.InNum`))
          (`KismetSystemLibrary.PrintString` (`KismetStringLibrary.Conv_IntToString` (`BlueprintMapLibrary.Map_Length` (`self.Medic`)))))))
    (:`NewEnumerator2`
      (if _returnvalue_3
        (bind _output_get_3 (set `local.ItemNum` _value_3))
        (`BlueprintMapLibrary.Map_Remove` _functional _inid_3)
        (`BlueprintMapLibrary.Map_Add` _functional _inid_3 (+ _output_get_3 (`local.InNum`)))
        (else
          (`BlueprintMapLibrary.Map_Add` (`self.Functional`) _inid_3 (`local.InNum`))
          (`KismetSystemLibrary.PrintString` (`KismetStringLibrary.Conv_IntToString` (`BlueprintMapLibrary.Map_Length` (`self.Functional`)))))))))

(fn `InsertToSubBag`
  (params (Id :type Integer) (SubBag :type "Map of Integer to Integer (by ref)"))
  (locals (SubBagToInsert :type "Map of Integer to Object Object Reference") (ItemNum :type Integer))
  (bind _subbagtoinsert (`local.SubBagToInsert`))
  (bind (_value _returnvalue) (`BlueprintMapLibrary.Map_Find` (`local.SubBagToInsert`)))
  (`|VariableSetRef` SubBag (`local.SubBagToInsert`))
  (if _returnvalue
    (bind _output_get (set `local.ItemNum` _value))
    (`BlueprintMapLibrary.Map_Remove` _subbagtoinsert Id)
    (`BlueprintMapLibrary.Map_Add` _subbagtoinsert Id (+ _output_get Id))
    (else
      (`BlueprintMapLibrary.Map_Add` (`local.SubBagToInsert`) Id Id)
      (`KismetSystemLibrary.PrintString` (`KismetStringLibrary.Conv_IntToString` (`BlueprintMapLibrary.Map_Length` (`local.SubBagToInsert`))))
      (`KismetSystemLibrary.PrintString` (`KismetStringLibrary.Conv_IntToString` (`BlueprintMapLibrary.Map_Length` (`self.Medic`)))))))

(fn `OutPutItems`
  (bind _functional (`self.Functional`))
  (bind _seeds (`self.Seeds`))
  (bind _medic (`self.Medic`))
  (`|ExecutionSequence`
    (:`then_0`
      (bind _keys (`BlueprintMapLibrary.Map_Keys` _functional))
      (for _array_element _keys
        (bind _res (`/Game/BluePrints/BP_Hero.Find Item Func` (`self.As BP Hero`) _array_element))
        (bind (_value _returnvalue) (`BlueprintMapLibrary.Map_Find` _functional _array_element))
        (if _returnvalue
          (`KismetSystemLibrary.PrintString` (`.Name_15_417A8145435FC759832FEB8C3406CBA0` (break `/Game/EnumsAndStructs/Item/Functional` _res)))
          (`KismetSystemLibrary.PrintString` (`KismetStringLibrary.Conv_IntToString` _value)))))
    (:`then_1`
      (bind _keys_2 (`BlueprintMapLibrary.Map_Keys` _seeds))
      (for _array_element_2 _keys_2
        (bind _res_2 (`/Game/BluePrints/BP_Hero.Find Item Medic` (`self.As BP Hero`) _array_element_2))
        (bind (_value_2 _returnvalue_2) (`BlueprintMapLibrary.Map_Find` _seeds _array_element_2))
        (if _returnvalue_2
          (`KismetSystemLibrary.PrintString` (`.Name_15_417A8145435FC759832FEB8C3406CBA0` (break `/Game/EnumsAndStructs/Item/Medi` _res_2)))
          (`KismetSystemLibrary.PrintString` (`KismetStringLibrary.Conv_IntToString` _value_2)))))
    (:`then_2`
      (bind _keys_3 (`BlueprintMapLibrary.Map_Keys` _medic))
      (for _array_element_3 _keys_3
        (bind _seed (`/Game/BluePrints/BP_Hero.Find Item Seed` (`self.As BP Hero`) _array_element_3))
        (bind (_value_3 _returnvalue_3) (`BlueprintMapLibrary.Map_Find` _medic _array_element_3))
        (if _returnvalue_3
          (`KismetSystemLibrary.PrintString` (`.Name_15_417A8145435FC759832FEB8C3406CBA0` (break `/Game/EnumsAndStructs/Item/Seed` _seed)))
          (`KismetSystemLibrary.PrintString` (`KismetStringLibrary.Conv_IntToString` _value_3)))))))

(fn `Remove`
  (params (id :type Integer) (num :type Integer) (type :type "/Game/EnumsAndStructs/Item/PropType Enum" :default "NewEnumerator0"))
  (returns (res :type Boolean))
  (bind _res (`self.CheckCanRemove` id num))
  (if _res
    (`self.Insert` id num type)
    (return true)
    (else
      (return false))))

(fn `UserConstructionScript`)