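; BP_PropBook is a manager Blueprint that serves as a lookup book for item props in three categories: seeds, medics and functionals.
; Each category has its own collection and a find function that returns the entry for a given Id.
; It holds no other logic, as its event graph and construction script are empty.
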(event `self.ReceiveBeginPlay`)

(fn `Find Item Func`
  (params (id :type Integer))
  (returns (NewParam1 :type "/Game/EnumsAndStructs/Item/Functional Structure"))
  (return (`|GetArrayItem` (`self.Functionals`) id)))

(fn `Find Item Seed`
  (params (id :type Integer))
  (returns (res :type "/Game/EnumsAndStructs/Item/Seed Structure"))
  (return (`|GetArrayItem` (`self.Seeds`) id)))

(fn `FindItemMedic`
  (params (id :type Integer))
  (returns (res :type "/Game/EnumsAndStructs/Item/Medi Structure"))
  (return (`|GetArrayItem` (`self.Medic`) id)))

(fn `UserConstructionScript`)