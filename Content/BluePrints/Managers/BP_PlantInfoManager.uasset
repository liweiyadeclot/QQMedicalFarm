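; BP_PlantInfoManager is a manager Blueprint that holds the static data for the game's plants: a sunflower entry and medicinal herbs such as licorice, ginger, coptis and ginseng.
; On BeginPlay it fills the SPlantsInfo array with hardcoded structs of type, grow time, seed, grown and medicine icons, and description.
; FindInfoByPlantType linearly searches that array and returns the matching entry, printing "NotFind!" when none matches.
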(event `self.ReceiveBeginPlay`
  (bind _s_plantsinfo (`self.s_PlantsInfo`))
  (`KismetArrayLibrary.Array_Insert` _s_plantsinfo (make `/Game/EnumsAndStructs/PlantsInfo` "NewEnumerator0" 0 "/Game/Resources/种田/图鉴_Sprite.图鉴_Sprite" "/Game/Resources/种田/收获_Sprite.收获_Sprite" "/Game/Resources/种田/播种_Sprite.播种_Sprite" "向日葵植物"))
  (`KismetArrayLibrary.Array_Insert` _s_plantsinfo (make `/Game/EnumsAndStructs/PlantsInfo` "NewEnumerator3" 3 "/Game/Resources/Plants/Seed/种子_甘草_Sprite.种子_甘草_Sprite" "/Game/Resources/Plants/Grown/植株_甘草_Sprite.植株_甘草_Sprite" "/Game/Resources/Plants/Medi/药材_甘草_Sprite.药材_甘草_Sprite" "甘草植物") 1)
  (`KismetArrayLibrary.Array_Insert` _s_plantsinfo (make `/Game/EnumsAndStructs/PlantsInfo` "NewEnumerator4" 3 "/Game/Resources/Plants/Seed/种子_生姜_Sprite.种子_生姜_Sprite" "/Game/Resources/Plants/Grown/植株_生姜_Sprite.植株_生姜_Sprite" "/Game/Resources/Plants/Medi/药材_生姜_Sprite.药材_生姜_Sprite" "甘草植物") 2)
  (`KismetArrayLibrary.Array_Insert` _s_plantsinfo (make `/Game/EnumsAndStructs/PlantsInfo` "NewEnumerator5" 0 "/Game/Resources/Plants/Seed/种子_黄连_Sprite.种子_黄连_Sprite" "/Game/Resources/Plants/Grown/植株_黄连_Sprite.植株_黄连_Sprite" "/Game/Resources/Plants/Medi/药材_黄连_Sprite.药材_黄连_Sprite" "甘草植物") 3)
  (`KismetArrayLibrary.Array_Insert` _s_plantsinfo (make `/Game/EnumsAndStructs/PlantsInfo` "NewEnumerator6" 0 "/Game/Resources/Plants/Seed/种子_人参_Sprite.种子_人参_Sprite" "/Game/Resources/Plants/Grown/植株_人参_Sprite.植株_人参_Sprite" "/Game/Resources/Plants/Medi/药材_人参_Sprite.药材_人参_Sprite" "甘草植物") 4))

(fn `FindInfoByPlantType`
  (params (input :type "/Game/EnumsAndStructs/Plants Enum" :default "NewEnumerator0"))
  (returns (NewParam :type "/Game/EnumsAndStructs/PlantsInfo Structure"))
  (for _array_element (`self.s_PlantsInfo`)
    (if (`|EnumEquality` (`.PlantsType_2_D6C2407946265171D00DD3A87ABAEA35` (break `/Game/EnumsAndStructs/PlantsInfo` _array_element)) input)
      (return _array_element)))
  (`KismetSystemLibrary.PrintString` "NotFind!"))

(fn `UserConstructionScript`)