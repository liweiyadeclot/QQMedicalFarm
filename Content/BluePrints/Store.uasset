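; Store is an Actor Blueprint with two clickable elements, one for travelling to the farm and one for showing the player's storage.
; On BeginPlay it caches the player's BP_Hero along with its game and grid manager references.
; Clicking ToFarm sets the game manager's current map, saves through the hero and opens the Farm level.
; Clicking Storage toggles the hero inventory's bag UI visibility through a FlipFlop.
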(event `self.ReceiveBeginPlay`
  (bind _asbp_hero (cast `/Game/BluePrints/BP_Hero` (`GameplayStatics.GetPlayerPawn` 0)))
  (set `self.HeroRef` _asbp_hero)
  (set `self.Game Manager Ref` (`/Game/BluePrints/BP_Hero.GameManagerRef` _asbp_hero))
  (set `self.Grid Manager Ref` (`/Game/BluePrints/BP_Hero.GridManagerRef` (`self.HeroRef`))))

(event `self.ToFarm.OnClicked`
  (params (TouchedComponent :type "PrimitiveComponent Object Reference") (ButtonPressed :type "Key Structure"))
  (set `/Game/BluePrints/Managers/BP_GameManager.curMap` "NewEnumerator1" (`self.Game Manager Ref`))
  (`/Game/BluePrints/BP_Hero.SaveGame` (`self.HeroRef`) false)
  (`GameplayStatics.OpenLevel` "Farm"))

(event `self.Storage.OnClicked`
  (params (TouchedComponent :type "PrimitiveComponent Object Reference") (ButtonPressed :type "Key Structure"))
  (bind _bagui (`/Game/BluePrints/InventoryComponent.BagUI` (`/Game/BluePrints/BP_Hero.InventoryComponent` (`self.HeroRef`))))
  (`/Engine/EditorBlueprintResources/StandardMacros.FlipFlop`
    (:`A`
      (`Widget.SetVisibility` _bagui "SelfHitTestInvisible"))
    (:`B`
      (`Widget.SetVisibility` _bagui "Hidden"))))

(fn `UserConstructionScript`)