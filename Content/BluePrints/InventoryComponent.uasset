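; Inventory component that holds the player's bag of props, seeds and plants, and grants four starter herb seeds on init.
; A fixed slot array is pre-filled with typed empty placeholders; AddItem merges stackables by name or takes that type's first empty slot, then refreshes BagUI.
; RemoveItem decrements or restores the placeholder, without refreshing the UI.
; Bag visibility switches input mode; throw and pickup are stubs, and BagUI creation is disconnected.
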(event `InitInventoryComponent`
  ;[1 1 1] Init
  (for _ (range 20)
    (`KismetArrayLibrary.Array_Add` (`self.ItemList`) (`self.EmptyProp`)))
  (for _ (range 20 110)
    (`KismetArrayLibrary.Array_Add` (`self.ItemList`) (`self.EmptySeed`)))
  (for _ (range 110 200)
    (`KismetArrayLibrary.Array_Add` (`self.ItemList`) (`self.EmptyPlant`)))
  (`self.AddItem` (make `/Game/EnumsAndStructs/BagItem` "甘草种子" "NewEnumerator0" true 1 "111" "/Game/Resources/Plants/Seed/种子_甘草_Sprite.种子_甘草_Sprite" null "NewEnumerator3"))
  (`self.AddItem` (make `/Game/EnumsAndStructs/BagItem` "黄连种子" "NewEnumerator0" true 1 "111" "/Game/Resources/Plants/Seed/种子_黄连_Sprite.种子_黄连_Sprite" null "NewEnumerator5"))
  (`self.AddItem` (make `/Game/EnumsAndStructs/BagItem` "生姜种子" "NewEnumerator0" true 1 "111" "/Game/Resources/Plants/Seed/种子_生姜_Sprite.种子_生姜_Sprite" null "NewEnumerator4"))
  (`self.AddItem` (make `/Game/EnumsAndStructs/BagItem` "人参种子" "NewEnumerator0" true 1 "111" "/Game/Resources/Plants/Seed/种子_人参_Sprite.种子_人参_Sprite" null "NewEnumerator6")))

(event `AddItem`
  (params (AddItem :type "/Game/EnumsAndStructs/BagItem Structure"))
  (bind (_itemname _itemtype _canstacking) (break `/Game/EnumsAndStructs/BagItem` AddItem))
  (bind (_itemname_2 _itemtype_2 _canstacking_2 _itemnumber) (break `/Game/EnumsAndStructs/BagItem` AddItem))
  (bind _itemlist (`self.ItemList`))
  (bind _itemlist_2 (`self.ItemList`))
  (bind _itemlist_3 (`self.ItemList`))
  (bind _itemlist_4 (`self.ItemList`))
  (bind _returnvalue (`KismetArrayLibrary.Array_Find` _itemlist (`self.EmptySeed`)))
  (bind _returnvalue_2 (`KismetArrayLibrary.Array_Find` _itemlist_2 (`self.EmptyProp`)))
  (bind _returnvalue_3 (`KismetArrayLibrary.Array_Find` _itemlist_4 (`self.EmptyPlant`)))
  ;[1 1 1] AddItem
  (if _canstacking
    (for (_array_element _array_index) _itemlist_3
      (bind (_itemname_3 _itemtype_3 _canstacking_3 _itemnumber_2) (break `/Game/EnumsAndStructs/BagItem` _array_element))
      (if (== _itemname_3 _itemname_2)
        (setmembers `/Game/EnumsAndStructs/BagItem` :`StructRef` (`|GetArrayItem` _itemlist_3 _array_index) :`ItemNumber` (+ _itemnumber_2 _itemnumber))
        (set `self.Flag` true)
        (break))))
  (if (`self.Flag`)
    (set `self.Flag` false :!label _label)
    (`/Game/UI/W_Bag.UpdateItemList` (`self.BagUI`))
    (else
      (switch `/Game/EnumsAndStructs/BagItemType` _itemtype
        (:`NewEnumerator0`
          (if (== _returnvalue -1)
            (`KismetSystemLibrary.PrintString` "背包已满")
            (else
              (`|VariableSetRef` (`|GetArrayItem` _itemlist _returnvalue) AddItem)
              (goto _label))))
        (:`NewEnumerator1`
          (if (== _returnvalue_2 -1)
            (`KismetSystemLibrary.PrintString` "背包已满")
            (else
              (`|VariableSetRef` (`|GetArrayItem` _itemlist_2 _returnvalue_2) AddItem)
              (goto _label))))
        (:`NewEnumerator2`
          (if (== _returnvalue_3 -1)
            (`KismetSystemLibrary.PrintString` "背包已满")
            (else
              (`|VariableSetRef` (`|GetArrayItem` _itemlist_4 _returnvalue_3) AddItem)
              (goto _label))))))))

(event `RemoveItem`
  (params (Index :type Integer) (Number :type Integer))
  (bind _output (`|GetArrayItem` (`self.ItemList`) Index))
  (bind (_itemname _itemtype _canstacking _itemnumber _discription _icon _mesh) (break `/Game/EnumsAndStructs/BagItem` _output))
  ;[1 1 1] RemoveItem
  (if (<= Number 0)
    _
    (elif (>= Number _itemnumber)
      (switch `/Game/EnumsAndStructs/BagItemType` _itemtype
        (:`NewEnumerator0`
          (`|VariableSetRef` _output (`self.EmptySeed`)))
        (:`NewEnumerator1`
          (`|VariableSetRef` _output (`self.EmptyProp`)))
        (:`NewEnumerator2`
          (`|VariableSetRef` _output (`self.EmptyPlant`))))
      (else
        (setmembers `/Game/EnumsAndStructs/BagItem` :`StructRef` _output :`ItemNumber` (- _itemnumber Number))))))

(event `ThrowItem`
  (params (Item :type "/Game/EnumsAndStructs/BagItem Structure")))

(event `self.ReceiveBeginPlay`
  (`|ExecutionSequence`
    (:`then_0`
      (bind _asplayer_controller (cast `PlayerController` (`Pawn.GetController` (`GameplayStatics.GetPlayerPawn` 0))))
      (set `self.PlayerController` _asplayer_controller))))

(event `SetInventoryUIVisiblity`
  (params (Visible :type Boolean))
  (bind _bagui (`self.BagUI`))
  (bind _playercontroller (`self.PlayerController`))
  (if Visible
    (`Widget.SetVisibility` _bagui "Visible")
    (`WidgetBlueprintLibrary.SetInputMode_GameAndUIEx` _playercontroller _bagui)
    (else
      (`Widget.SetVisibility` _bagui "Hidden")
      (`WidgetBlueprintLibrary.SetInputMode_GameOnly` _playercontroller))))

(event `InputPickUpItem`)